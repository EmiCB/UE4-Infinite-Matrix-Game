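; BP_Enemy is an enemy actor that damages the player on contact and awards score when shot.
; Overlap on its Cone component either applies damage through the player's UpdateHealth, or on a BP_Projectile hit increments the player's score and destroys the projectile.
; Both overlap outcomes destroy the enemy.
; Tick also destroys it once the player's X position exceeds its own, cleaning up enemies the player has passed.
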(event `self.ReceiveTick`
  (params (DeltaSeconds :type "Float (single-precision)"))
  ;[1 1 1] Destroy after player passes
  (bind _asbp_player (cast `/Game/InfiniteMatrix/Blueprints/BP_Player` (`GameplayStatics.GetPlayerPawn` 0)))
  (if (> (.x (.location (`self.GetTransform` _asbp_player))) (.x (.location (`self.GetTransform`))))
    (`self.K2_DestroyActor`)))

(event `self.Cone.OnComponentBeginOverlap`
  (params (OverlappedComponent :type "PrimitiveComponent Object Reference") (OtherActor :type "Actor Object Reference") (OtherComp :type "PrimitiveComponent Object Reference") (OtherBodyIndex :type Integer) (bFromSweep :type Boolean) (SweepResult :type "HitResult Structure (by ref)"))
  ;[1 1 1] OnComponentBeginOverlap
  ;;[1 1 1] Damage player when hit
  (bind _asbp_player (cast `/Game/InfiniteMatrix/Blueprints/BP_Player` OtherActor)
    (:`then`
      (`/Game/InfiniteMatrix/Blueprints/BP_Player.UpdateHealth` _asbp_player (`self.Damage`)))
    (:`CastFailed`
      ;;[1 1 1] Projectile destroys and adds points
      (bind _asbp_projectile (cast `/Game/InfiniteMatrix/Blueprints/BP_Projectile` OtherActor))
      (bind _asbp_player_2 (cast `/Game/InfiniteMatrix/Blueprints/BP_Player` (`GameplayStatics.GetPlayerPawn` 0)))
      (`/Game/InfiniteMatrix/Blueprints/BP_Player.IncrementScore` _asbp_player_2 (`self.ScoreValue`))
      (`self.K2_DestroyActor` _asbp_projectile)))
  (`self.K2_DestroyActor`))

(fn `UserConstructionScript`)