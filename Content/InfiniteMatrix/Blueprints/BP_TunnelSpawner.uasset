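; BP_TunnelSpawner builds a chain of tunnel segments, starting with three at BeginPlay.
; The first spawns at the player pawn's location; each following one spawns at the SpawnPoint of NewestTunnel, the last one spawned.
; Every new tunnel receives a reference back to the spawner and randomizes its obstacle wall.
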(event `self.ReceiveBeginPlay`
  ;[1 1 1] Spawn initial tunnels
  (`self.SpawnInitialTunnels`))

(fn `SpawnInitialTunnels`
  ;[1 1 1] set up initial 3 tunnels
  (for _ (range 3)
    (`/Engine/EditorBlueprintResources/StandardMacros.IsValid` (`self.NewestTunnel`)
      (:`Is Valid`
        ;;[1 1 1] spawn other tunnels
        (`self.SpawnTunnelAtSpawnPoint`))
      (:`Is Not Valid`
        ;;[1 1 1] spawn initial tunnel on player location
        (`self.SpawnTunnel` (`self.K2_GetActorLocation` (`GameplayStatics.GetPlayerPawn` 0)))))))

(fn `SpawnTunnel`
  (params (SpawnLocation :type "Vector Structure"))
  ;[1 1 1] Spawns a tunnel at the given location, randomizes obstacle wall
  (bind _returnvalue (`|SpawnActorFromClass` "/Game/InfiniteMatrix/Blueprints/BP_Tunnel.BP_Tunnel_C" (`KismetMathLibrary.MakeTransform` SpawnLocation) "Undefined" "OverrideRootScale" null null))
  (bind _output_get (set `self.NewestTunnel` _returnvalue))
  (set `/Game/InfiniteMatrix/Blueprints/BP_Tunnel.TunnelSpawner` self _output_get)
  (`/Game/InfiniteMatrix/Blueprints/BP_Tunnel.RandomizeWall` _returnvalue))

(fn `SpawnTunnelAtSpawnPoint`
  ;[1 1 1] Spawn tunnel at last tunnel spawn point
  (`self.SpawnTunnel` (`SceneComponent.K2_GetComponentLocation` (`/Game/InfiniteMatrix/Blueprints/BP_Tunnel.SpawnPoint` (`self.NewestTunnel`)))))

(fn `UserConstructionScript`)